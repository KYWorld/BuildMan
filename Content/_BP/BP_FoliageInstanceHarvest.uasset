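; Foliage instance component that lets the player harvest trees by chopping individual instances.
; After a short delay on BeginPlay, it caches the player's inventory component and fills a health array indexed by instance.
; Chop damages the hit instance and, using a data table row, adds a random amount of that item to the inventory on every hit.
; At zero health it plays a break sound and removes the instance, leaving the health array unchanged.
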(event EventBeginPlay
  ;[0.1493 0.1493 0.1493] Set Initial Health
  (Utilities|FlowControl|Delay 0.2)
  (bind _asbp_third_person_character (Utilities|Casting|CastToBP_ThirdPersonCharacter (Game|GetPlayerCharacter 0)))
  (Variables|Default|SetBPC%20Inventory%20Component (Variables|/Game/ThirdPerson/Blueprints/BP_ThirdPersonCharacter.BP_ThirdPersonCharacter_C|GetBPC_InventoryComponent _asbp_third_person_character))
  (for _index (range 0 (Components|InstancedStaticMesh|GetInstanceCount))
    (Utilities|Array|SetArrayElem (Variables|Default|GetFoliageHealth) _index (Utilities|Struct|MakeST_FoliageHealth 5.0) true)))

(event EventChop
  (params (Damage :type Float%20%28double-precision%29) (Hit :type Hit%20Result%20Structure))
  (bind _hititem (Collision|BreakHitResult Hit))
  (bind _foliagehealth (Variables|Default|GetFoliageHealth))
  (bind _datatablerow (Variables|Default|GetDataTableRow))
  (bind _output (Utilities|Array|Get(acopy) _foliagehealth _hititem))
  (bind _returnvalue (- (.health _output) Damage))
  ;[0.1493 0.1493 0.1493] Chop Tree
  (Utilities|Array|SetArrayElem (Variables|Default|GetFoliageHealth) _hititem (Utilities|Struct|MakeST_FoliageHealth _returnvalue))
  (bind _returnvalue_2 (Utilities|GetDataTableRow (.datatable _datatablerow) (.rowname _datatablerow))
    (:then
      (Default|AddItem (Variables|Default|GetBPC%20Inventory%20Component) (Utilities|Struct|MakeST_Item (.Name (Utilities|Struct|BreakST_Item _returnvalue_2)) (Math|Random|RandomIntegerinRange 2 5) (.Mesh (Utilities|Struct|BreakST_Item _returnvalue_2)) (.Icon (Utilities|Struct|BreakST_Item _returnvalue_2)) (.CanCraft (Utilities|Struct|BreakST_Item _returnvalue_2))))
      (if (<= _returnvalue 0.0)
        (Audio|SpawnSoundatLocation "/Game/Audio/Sound/MS_TreeBreak.MS_TreeBreak" (.location (.OutInstanceTransform (Components|InstancedStaticMesh|GetInstanceTransform _hititem true))) "0, 0, 0" 1.0 1.0 0.0 0 0)
        (Class|InstancedStaticMeshComponent|RemoveInstance _hititem)))))