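; BP_Item is an inventory item actor that represents a pickup in the world, configured from the DT_Item data table.
; The construction script looks up the assigned ItemRow, or randomly Wood or Stone when RandomItem is set, then stores the row and applies its mesh.
; PickupItem returns the stored item and always allows pickup, without removing the actor itself.
; Event graph events are empty.
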(event EventBeginPlay)

(event Collision|EventActorBeginOverlap
  (params (OtherActor :type Actor%20Object%20Reference)))

(event EventTick
  (params (DeltaSeconds :type Float%20%28single-precision%29)))

(fn ConstructionScript
  (if (not (Variables|Default|GetRandomItem))
    (bind _returnvalue (Utilities|GetDataTableRow "/Game/_BP/Inventory/DT_Item.DT_Item" (.rowname (Variables|Default|GetItemRow)))
      (:then
        (Variables|Default|SetItem _returnvalue)))
    (else
      (bind _returnvalue_2 (Utilities|GetDataTableRow "/Game/_BP/Inventory/DT_Item.DT_Item" (.OutItem (Utilities|Array|Random (Utilities|Array|MakeArray "Wood" "Stone"))))
        (:then
          (Variables|Default|SetItem _returnvalue_2)))))
  (Components|StaticMesh|SetStaticMesh (Variables|Default|GetStaticMesh) (.Mesh (Utilities|Struct|BreakST_Item (Variables|Default|GetItem)))))

(fn PickupItem
  (return (Variables|Default|GetItem) true))