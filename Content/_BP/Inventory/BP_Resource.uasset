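; BP_Resource is a harvestable resource actor that yields inventory items when damaged.
; Damage from a causer implementing BPI_Inventory lowers Health, and the actor is destroyed once it is depleted.
; Each surviving hit picks a random entry from Items, looks it up in DT_Item, and sends the causer that item with a random amount through HarvestItemMessage, so the destroying hit yields nothing.
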(event Game|Damage|EventAnyDamage
  (params (Damage :type Float%20%28single-precision%29) (DamageType :type Damage%20Type%20Object%20Reference) (InstigatedBy :type Controller%20Object%20Reference) (DamageCauser :type Actor%20Object%20Reference))
  (if (Utilities|DoesObjectImplementInterface DamageCauser "/Game/_BP/Interface/BPI_Inventory.BPI_Inventory_C")
    (bind _output_get (Variables|Default|SetHealth (- (Variables|Default|GetHealth) Damage)))
    (if (<= _output_get 0.0)
      (Actor|DestroyActor)
      (else
        (bind _returnvalue (Utilities|GetDataTableRow "/Game/_BP/Inventory/DT_Item.DT_Item" (.rowname (.OutItem (Utilities|Array|Random (Variables|Default|GetItems)))))
          (:then
            (Class|BPIInventory|HarvestItem(Message) DamageCauser (Utilities|Struct|MakeST_Item (.Name (Utilities|Struct|BreakST_Item _returnvalue)) (Math|Random|RandomIntegerinRange 2 5) (.Mesh (Utilities|Struct|BreakST_Item _returnvalue)) (.Icon (Utilities|Struct|BreakST_Item _returnvalue)) (.CanCraft (Utilities|Struct|BreakST_Item _returnvalue)) (.ResourceNeeded (Utilities|Struct|BreakST_Item _returnvalue))))))))))

(fn ConstructionScript)