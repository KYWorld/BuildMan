(event Custom|BuildMode
  (bind _buildpart (Variables|Default|GetBuildPart))
  ;[0.1493 0.1493 0.1493] Enter Build Mode
  (Variables|Default|SetInBuildMode true)
  (bind _returnvalue (Game|AddComponentbyClass (Components|GetOwner) "/Script/Engine.StaticMeshComponent" false))
  (bind _returnvalue_2 (Utilities|GetDataTableRow (.datatable _buildpart) (.rowname _buildpart))
    (:then
      (Components|StaticMesh|SetStaticMesh _returnvalue (.Mesh (Utilities|Struct|BreakST_BuildPart _returnvalue_2)))
      (Collision|SetCollisionEnabled _returnvalue "NoCollision")
      (Rendering|Material|SetMaterial _returnvalue 0 "/Game/Material/MAT_BuildPreview.MAT_BuildPreview")
      (Variables|Default|SetBuildPreviewMesh _returnvalue))))

(event Custom|StopBuildMode
  (bind _buildpreviewmesh (Variables|Default|GetBuildPreviewMesh))
  ;[0.1493 0.1493 0.1493] Build Preview Stop
  (Variables|Default|SetInBuildMode false)
  (Components|StaticMesh|SetStaticMesh _buildpreviewmesh 0)
  (Components|DestroyComponent _buildpreviewmesh))

(event Input|EnhancedActionEvents|EnhancedInputActionIA_Attack
  (params (ActionValue :type Boolean) (ElapsedSeconds :type Float%20%28double-precision%29) (TriggeredSeconds :type Float%20%28double-precision%29) (InputAction :type Input%20Action%20Object%20Reference :default "/Game/ThirdPerson/Input/Actions/IA_Attack.IA_Attack"))
  (bind _buildpart (Variables|Default|GetBuildPart))
  (bind _buildpreviewmesh (Variables|Default|GetBuildPreviewMesh))
  (bind _returnvalue (Transformation|GetWorldTransform _buildpreviewmesh))
  ;[0.1493 0.1493 0.1493] Build Placement
  (:Started
    (if (Variables|Default|GetInBuildMode)
      (bind _returnvalue_2 (Utilities|GetDataTableRow (.datatable _buildpart) (.rowname _buildpart))
        (:then
          (Game|SpawnActorfromClass (.Actor (Utilities|Struct|BreakST_BuildPart _returnvalue_2)) (Math|Transform|MakeTransform (.location _returnvalue) (.rotation _returnvalue) "1.000000,1.000000,1.000000") "AlwaysSpawn" "MultiplyWithRoot" 0 0))))))

(event EventBeginPlay
  ;[0.1493 0.1493 0.1493] Begin Play
  (bind _asbp_third_person_character (Utilities|Casting|CastToBP_ThirdPersonCharacter (Components|GetOwner)))
  (Variables|Default|SetPlayer _asbp_third_person_character)
  (CallFunction|BuildMode))

(event EventTick
  (params (DeltaSeconds :type Float%20%28single-precision%29))
  ;[0.1493 0.1493 0.1493] Build Preview Update
  (if (Variables|Default|GetInBuildMode)
    (bind (_hit _location) (CallFunction|LineTrace))
    (if _hit
      (Transformation|SetWorldLocationAndRotation (Variables|Default|GetBuildPreviewMesh) _location (Transformation|GetActorRotation (Components|GetOwner)) false false))))

(fn LineTrace
  (bind _returnvalue (Game|GetPlayerCameraManager 0))
  (bind _returnvalue_2 (Transformation|GetActorLocation _returnvalue))
  (bind _returnvalue_3 (Transformation|GetActorRotation _returnvalue))
  (bind _returnvalue_4 (Math|Vector|GetForwardVector _returnvalue_3))
  (bind (_outhit _returnvalue_5) (Collision|LineTraceByChannel (+ _returnvalue_2 (* _returnvalue_4 7e+02)) (+ _returnvalue_2 (* _returnvalue_4 1e+03)) "TraceTypeQuery1" false 0 "None"))
  (return _returnvalue_5 (Math|Vector|SelectVector (.Location (Collision|BreakHitResult _outhit)) "0, 0, 0" _returnvalue_5)))