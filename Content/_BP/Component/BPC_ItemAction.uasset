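; Actor component on the third-person character that handles the player's melee attack and harvesting.
; The attack input plays a montage with a whoosh, blocked while the inventory widget is valid or until the previous swing completes or is interrupted.
; On the montage notify, a forward sphere trace applies damage, spawns hit effects and sound, and sends a chop message to hit components implementing the foliage interaction interface.
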(event Custom|AttackAndHarvest
  (bind _player (Variables|Default|GetPlayer))
  (bind _returnvalue (Transformation|GetActorLocation _player))
  (bind _returnvalue_2 (Transformation|GetActorRotation _player))
  (bind _returnvalue_3 (Math|Vector|GetForwardVector _returnvalue_2))
  (Variables|Default|GetInventory%20Widget
    (:then)
    (:else
      (if (Variables|Default|GetCanAttack)
        (Animation|Montage|PlayMontage (Variables|/Script/Engine.Character|GetMesh (Variables|Default|GetPlayer)) "/Game/Characters/Mannequins/Animations/Manny/MM_Attack_Montage.MM_Attack_Montage"
          (:then
            (Variables|Default|SetCanAttack false)
            (Audio|PlaySoundatLocation "/Game/Audio/Sound/MS_Whoosh.MS_Whoosh" (Transformation|GetActorLocation (Components|GetOwner)) "0, 0, 0" 1.0 1.0 0.0 0 0 0 0))
          (:OnCompleted
            (Variables|Default|SetCanAttack true :!label _label))
          (:OnInterrupted
            (goto _label))
          (:OnNotifyBegin
            (bind (_outhit _returnvalue_4) (Collision|SphereTraceForObjects (+ _returnvalue (* _returnvalue_3 1.0)) (+ _returnvalue (* _returnvalue_3 2.5e+02)) 55.0 (Utilities|Array|MakeArray "ObjectTypeQuery2" "ObjectTypeQuery1" "ObjectTypeQuery3") false (Utilities|Array|MakeArray (Components|GetOwner)) "ForDuration"))
            (if _returnvalue_4
              (Game|Damage|ApplyDamage (.HitActor (Collision|BreakHitResult _outhit)) 1e+01 0 (Components|GetOwner))
              (Niagara|SpawnSystematLocation "/Game/NiagaraEffect/NS_Hit.NS_Hit" (.Location (Collision|BreakHitResult _outhit)) "0, 0, 0" "1.000000,1.000000,1.000000" true true "AutoRelease")
              (Audio|PlaySoundatLocation "/Game/Audio/Sound/MS_Hit.MS_Hit" (.Location (Collision|BreakHitResult _outhit)) "0, 0, 0" 1.0 1.0 0.0 0 0 0 0)
              (if (Utilities|DoesObjectImplementInterface (.HitComponent (Collision|BreakHitResult _outhit)) "/Game/_BP/Interface/BPI_FoliageInteraction.BPI_FoliageInteraction_C")
                (Class|BPIFoliageInteraction|Chop(Message) (.HitComponent (Collision|BreakHitResult _outhit)) 1.0 _outhit)))))))))

(event Input|EnhancedActionEvents|EnhancedInputActionIA_Attack
  (params (ActionValue :type Boolean) (ElapsedSeconds :type Float%20%28double-precision%29) (TriggeredSeconds :type Float%20%28double-precision%29) (InputAction :type Input%20Action%20Object%20Reference :default "/Game/ThirdPerson/Input/Actions/IA_Attack.IA_Attack"))
  (:Triggered
    (CallFunction|AttackandHarvest)))

(event EventBeginPlay
  ;[0.1493 0.1493 0.1493] Initialize Variables
  (bind _asbp_third_person_character (Utilities|Casting|CastToBP_ThirdPersonCharacter (Components|GetOwner)))
  (Variables|Default|SetPlayer _asbp_third_person_character)
  (Variables|Default|SetBPC%20Inventory%20Component (Variables|/Game/ThirdPerson/Blueprints/BP_ThirdPersonCharacter.BP_ThirdPersonCharacter_C|GetBPC_InventoryComponent (Variables|Default|GetPlayer)))
  (Variables|Default|SetInventory%20Widget (Variables|/Game/_BP/Component/BPC_InventoryComponent.BPC_InventoryComponent_C|GetInventoryWidget (Variables|Default|GetBPC%20Inventory%20Component))))